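; AI_Centipede is a centipede enemy character driven by an EnemyAIController.
; On BeginPlay it passes its Behaviour to the controller, initializes the AI and sets walk speed.
; A hit trigger overlapping the ThirdPersonCharacter only prints "Kill Player" for now.
; The Death function subtracts damage from Health and, at zero or below, spawns a pixel explosion, logs the death and destroys the actor.
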(event OnComponentBeginOverlap(HitTrigger)
  (params (OverlappedComponent :type Primitive%20Component%20Object%20Reference) (OtherActor :type Actor%20Object%20Reference) (OtherComp :type Primitive%20Component%20Object%20Reference) (OtherBodyIndex :type Integer) (bFromSweep :type Boolean) (SweepResult :type Hit%20Result%20Structure%20%28by%20ref%29))
  (Utilities|Casting|CastToThirdPersonCharacter OtherActor)
  (Development|PrintString "Kill Player"))

(event EventBeginPlay
  (bind _asenemy_aicontroller (Utilities|Casting|CastToEnemyAIController (Pawn|GetController)))
  (Variables|/Game/BluePrints/AI/EnemyAIController.EnemyAIController_C|SetBehaviour _asenemy_aicontroller (Variables|Default|Getbehaviour))
  (Default|InitializeAI _asenemy_aicontroller)
  (Variables|/Script/Engine.CharacterMovementComponent|SetMaxWalkSpeed (Variables|Character|GetCharacterMovement) (Variables|Default|GetWalk_Speed)))

(event Collision|EventActorBeginOverlap
  (params (OtherActor :type Actor%20Object%20Reference)))

(event EventTick
  (params (DeltaSeconds :type Float%20%28single-precision%29)))

(fn ConstructionScript)

(fn Death
  (params (Damage :type Float%20%28single-precision%29))
  (bind _self self)
  (bind _output_get (Variables|Default|SetHealth (- (Variables|Default|GetHealth) Damage)))
  (if (<= _output_get 0.0)
    (Effects|SpawnEmitteratLocation "/Game/Assests/ParticleEffects/EnemyDeath/P_PixelExp.P_PixelExp" (Transformation|GetActorLocation _self) (Transformation|GetActorRotation _self) "0.250000,0.250000,0.250000")
    (Development|PrintString (Utilities|String|Append (Utilities|GetDisplayName _self) " has died!"))
    (Actor|DestroyActor)))