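; Spider enemy character driven by an EnemyAIController and a shared AIComponent.
; On BeginPlay it hands its Behaviour to the controller, initializes the AI, sets walk speed, and seeds the component with owner, type and starting health.
; Damage is forwarded to the AIComponent.
; HitTrigger overlap with the ThirdPersonCharacter only prints "Kill Player", with no kill logic yet.
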(event OnComponentBeginOverlap(HitTrigger)
  (params (OverlappedComponent :type Primitive%20Component%20Object%20Reference) (OtherActor :type Actor%20Object%20Reference) (OtherComp :type Primitive%20Component%20Object%20Reference) (OtherBodyIndex :type Integer) (bFromSweep :type Boolean) (SweepResult :type Hit%20Result%20Structure%20%28by%20ref%29))
  ;[1 0 0] Kill Player
  (Utilities|Casting|CastToThirdPersonCharacter OtherActor)
  (Development|PrintString "Kill Player"))

(event EventBeginPlay
  (bind _aicomponent (Variables|Default|GetAIComponent))
  (bind _asenemy_aicontroller (Utilities|Casting|CastToEnemyAIController (Pawn|GetController))
    (:then
      (Variables|/Game/BluePrints/AI/EnemyAIController.EnemyAIController_C|SetBehaviour _asenemy_aicontroller (Variables|Default|Getbehaviour))
      (Default|InitializeAI _asenemy_aicontroller)
      (Variables|/Script/Engine.CharacterMovementComponent|SetMaxWalkSpeed (Variables|Character|GetCharacterMovement) (Variables|Default|GetWalk_Speed))
      (Variables|/Game/BluePrints/AI/AIComponent.AIComponent_C|SetParentObject _aicomponent self)
      (Variables|/Game/BluePrints/AI/AIComponent.AIComponent_C|SetAIType _aicomponent "NewEnumerator1")
      (Variables|/Game/BluePrints/AI/AIComponent.AIComponent_C|SetHealth _aicomponent (Variables|Default|GetInitHealth)))
    (:CastFailed
      (Development|PrintString "Player Not found"))))

(event Collision|EventActorBeginOverlap
  (params (OtherActor :type Actor%20Object%20Reference)))

(event EventTick
  (params (DeltaSeconds :type Float%20%28single-precision%29)))

(event EventTakeDamage
  (params (Damage :type Float%20%28single-precision%29))
  (Default|DamageAI (Variables|Default|GetAIComponent) Damage))

(fn ConstructionScript)