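; CentipedePartController is an AI controller for centipede parts that gives each one a target object to act on through a behavior tree.
; On BeginPlay it initializes the CentipedeBB blackboard, writes TargetObject to the key named by TargetObjectName, then runs the Behaviour tree, with debug prints along the way.
; The UpdateTarget event overwrites that blackboard key with a new target at runtime.
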(event Custom|UpdateTarget
  (params (NewTarget :type Character%20Object%20Reference))
  (AI|Components|Blackboard|SetValueasObject (AI|GetBlackboard self) (Variables|Default|GetTargetObjectName) NewTarget))

(event EventBeginPlay
  (bind _targetobject (Variables|Default|GetTargetObject))
  (Development|PrintString "AI Initializing")
  (bind _blackboardcomponent (Class|AIController|UseBlackboard "/Game/BluePrints/AI/CentipedeBB.CentipedeBB"))
  (Development|PrintString (Utilities|GetDisplayName _targetobject))
  (AI|Components|Blackboard|SetValueasObject _blackboardcomponent (Variables|Default|GetTargetObjectName) _targetobject)
  (AI|RunBehaviorTree (Variables|Default|GetBehaviour)))

(event EventTick
  (params (DeltaSeconds :type Float%20%28single-precision%29)))

(fn ConstructionScript)