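; AI controller for enemy characters that starts their behavior tree when play begins.
; On BeginPlay it sets up the EnemyBB blackboard, stores the first player character in the PlayerCharacter key, then runs the Behaviour tree, printing debug messages along the way.
; An Initialize AI function duplicates the same setup logic but is not called within this Blueprint.
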(event EventBeginPlay
  (bind _returnvalue (Game|GetPlayerCharacter 0))
  (Development|PrintString "AI Initializing")
  (bind _blackboardcomponent (Class|AIController|UseBlackboard "/Game/BluePrints/AI/EnemyBB.EnemyBB"))
  (Development|PrintString (Utilities|GetDisplayName _returnvalue))
  (AI|Components|Blackboard|SetValueasObject _blackboardcomponent (Variables|Default|GetPlayer%20Character) _returnvalue)
  (AI|RunBehaviorTree (Variables|Default|GetBehaviour)))

(event EventTick
  (params (DeltaSeconds :type Float%20%28single-precision%29)))

(fn ConstructionScript)

(fn InitializeAI
  (bind _returnvalue (Game|GetPlayerCharacter 0))
  (Development|PrintString "AI Initializing")
  (bind _blackboardcomponent (Class|AIController|UseBlackboard "/Game/BluePrints/AI/EnemyBB.EnemyBB"))
  (Development|PrintString (Utilities|GetDisplayName _returnvalue))
  (AI|Components|Blackboard|SetValueasObject _blackboardcomponent (Variables|Default|GetPlayer%20Character) _returnvalue)
  (AI|RunBehaviorTree (Variables|Default|GetBehaviour)))