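; Behavior tree task that steps an AI pawn toward the closest BP_Player1 actor.
; On execute, it loops over all such actors, keeping the nearest location, with -1 distance meaning none found yet.
; It projects a point a short fixed step toward that location, at a hardcoded height, onto the navmesh and runs AI MoveTo.
; The task succeeds when the move completes and fails if projection or movement fails.
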(event EventReceiveExecuteAI
  (params (OwnerController :type AI%20Controller%20Object%20Reference) (ControlledPawn :type Pawn%20Object%20Reference))
  (bind _returnvalue (Transformation|GetActorLocation ControlledPawn))
  (bind _outactors (Actor|GetAllActorsOfClass "/Game/ThirdPersonBP/Blueprints/BP_Player1.BP_Player1_C"))
  ;[1 1 1] Loop (Find Closest Target)
  (for _array_element _outactors
    (if (Utilities|IsValid _array_element)
      (if (== (Variables|Default|GetClosestPlayerDistance) -1.0)
        (Variables|Default|SetClosestPlayer (Transformation|GetActorLocation _array_element) :!label _label)
        (Variables|Default|SetClosestPlayerDistance (Math|Float|Absolute(Float) (Math|Vector|VectorLength (- (Transformation|GetActorLocation _array_element) _returnvalue))))
        (elif (>= (Variables|Default|GetClosestPlayerDistance) (Math|Float|Absolute(Float) (Math|Vector|VectorLength (- (Transformation|GetActorLocation _array_element) _returnvalue))))
          (goto _label)))
      (elif (== (Variables|Default|GetClosestPlayerDistance) -1.0)
        (Development|PrintString "NotTargetsFound")
        (else
          (Development|PrintString "Invalid Owner")))))
  ;[0 0.3813 0.8632] Move AI to Closest Target
  (if (.ReturnValue (AI|Navigation|ProjectPointtoNavigation (Math|Vector|MakeVector (.X (Math|Vector|BreakVector (+ (* (Math|Vector|Normalize (- (Variables|Default|GetClosestPlayer) _returnvalue)) 1.5e+02) _returnvalue))) (.Y (Math|Vector|BreakVector (+ (* (Math|Vector|Normalize (- (Variables|Default|GetClosestPlayer) _returnvalue)) 1.5e+02) _returnvalue))) 42.0) 0 0 "0.000000,0.000000,0.000000"))
    (AI|AIMoveTo ControlledPawn (.ProjectedLocation (AI|Navigation|ProjectPointtoNavigation (Math|Vector|MakeVector (.X (Math|Vector|BreakVector (+ (* (Math|Vector|Normalize (- (Variables|Default|GetClosestPlayer) _returnvalue)) 1.5e+02) _returnvalue))) (.Y (Math|Vector|BreakVector (+ (* (Math|Vector|Normalize (- (Variables|Default|GetClosestPlayer) _returnvalue)) 1.5e+02) _returnvalue))) 42.0) 0 0 "0.000000,0.000000,0.000000")) 0 1.0 false
      (:OnSuccess
        (AI|BehaviorTree|FinishExecute true))
      (:OnFail
        (Development|PrintString "Failed to Find/Reach Target")
        (AI|BehaviorTree|FinishExecute false :!label _label_2)))
    (else
      (Development|PrintString "Failed to Find/Reach Nav Target")
      (goto _label_2))))