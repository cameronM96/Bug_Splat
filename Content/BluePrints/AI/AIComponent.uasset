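; Shared AI component that manages enemy health, hit effects, burning and death.
; DamageAI subtracts health and, at zero, adds score through the GameModeController before Death removes the AI from the game mode and destroys it.
; SetFire attaches a flame emitter and starts timed burn damage, paced by a Delay on Tick, with extra body-part removal for centipedes.
; Startup retries the game mode cast, calling Death after repeated failures.
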(event Custom|PutOutFire
  (Variables|Default|SetOnFire false)
  (Components|DestroyComponent (Variables|Default|GetFireEffect))
  (Variables|Default|SetFireEffect 0))

(event Custom|Death
  (params (Parent :type Pawn%20Object%20Reference))
  (if (Utilities|IsValid Parent)
    (Variables|Default|SetKilled true)
    (Effects|SpawnEmitteratLocation "/Game/Assests/ParticleEffects/EnemyDeath/P_PixelExp.P_PixelExp" (Transformation|GetActorLocation Parent) (Transformation|GetActorRotation Parent) "0.150000,0.150000,0.150000")
    (Class|BPIAI|RemoveAI(Message) (Game|GetGameMode) Parent)
    (Utilities|FlowControl|Delay 0.2)
    (Actor|DestroyActor Parent)
    (else
      (Development|PrintString "NoParentFound"))))

(event Custom|ReInitialise
  (if (<= (Variables|Default|GetFails) 3)
    (Utilities|FlowControl|Delay 0.2)
    (bind _asgame_mode_controller (Utilities|Casting|CastToGameModeController (Game|GetGameMode))
      (:then
        (Variables|Default|SetGamemode _asgame_mode_controller))
      (:CastFailed
        (Development|PrintString "Gamemode Not Found!")
        (Math|Integer|IncrementInt (Variables|Default|GetFails)
          (:%20%20
            (CallFunction|ReInitialise)))))
    (else
      (CallFunction|Death (Variables|Default|GetParentObject)))))

(event EventBeginPlay
  (if (<= (Variables|Default|GetFails) 3)
    (Utilities|FlowControl|Delay 0.2)
    (bind _asgame_mode_controller (Utilities|Casting|CastToGameModeController (Game|GetGameMode))
      (:then
        (Variables|Default|SetGamemode _asgame_mode_controller))
      (:CastFailed
        (Development|PrintString "Gamemode Not Found!")
        (Math|Integer|IncrementInt (Variables|Default|GetFails)
          (:%20%20
            (CallFunction|ReInitialise)))))
    (else
      (CallFunction|Death (Variables|Default|GetParentObject)))))

(event EventTick
  (params (DeltaSeconds :type Float%20%28single-precision%29))
  (bind _parentobject (Variables|Default|GetParentObject))
  (if (Variables|Default|GetOnFire)
    (Variables|Default|Settimer (- (Variables|Default|Gettimer) DeltaSeconds))
    (Utilities|FlowControl|Delay 1.0)
    (CallFunction|DamageAI (Variables|Default|GetFireDamage) _parentobject)
    (if (not (== (Utilities|GetClass _parentobject) "/Game/BluePrints/AI/AI_Centipede.AI_Centipede_C"))
      _
      (else
        (bind _asai_centipede (Utilities|Casting|CastToAI_Centipede (Variables|Default|GetParentObject))
          (:then
            (Default|CalcBodyPartRemoval _asai_centipede (Variables|Default|GetFireDamage)))
          (:CastFailed
            _))))
    (if (<= (Variables|Default|Gettimer) 0.0)
      (CallFunction|PutOutFire))))

(event EventSetFire
  (params (FireDamage :type Float%20%28single-precision%29) (FireDuraction :type Float%20%28single-precision%29))
  (Variables|Default|SetFireDamage FireDamage)
  (bind _output_get (Variables|Default|SetFireDuration FireDuraction))
  (Variables|Default|Settimer _output_get)
  (if (Utilities|IsValid (Variables|Default|GetFireEffect))
    _
    (else
      (Class|BPIAI|GetEmitterLocation(Message) (Variables|Default|GetParentObject))
      (bind _returnvalue (Effects|SpawnEmitterAttached "/Game/Assests/ParticleEffects/OnFire/OnFireReal.OnFireReal" (Variables|Default|GetEmitterAttachPoint) "None" "0, 0, 0" "0, 0, 0" "1.000000,1.000000,1.000000" "KeepRelativeOffset" false))
      (Variables|Default|SetFireEffect _returnvalue)))
  (Variables|Default|SetOnFire true))

(fn DamageAI
  (params (Damage :type Float%20%28single-precision%29) (Parent :type Pawn%20Object%20Reference))
  (bind _output_get (Variables|Default|SetParentObject Parent))
  (bind _output_get_2 (Variables|Default|SetHealth (- (Variables|Default|GetHealth) Damage)))
  (Effects|SpawnEmitteratLocation "/Game/Assests/ParticleEffects/EnemyHit/PS_EnemyHit.PS_EnemyHit" (Transformation|GetActorLocation Parent) (Transformation|GetActorRotation Parent) "0.150000,0.150000,0.150000")
  (if (and (<= _output_get_2 0.0) (not (Variables|Default|GetKilled)))
    ;[0.000304 0.3813 0.855] Add Score
    (Default|AddScore (Variables|Default|GetGamemode) (Variables|Default|GetAIType))
    (CallFunction|Death _output_get)))