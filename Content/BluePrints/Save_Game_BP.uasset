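; Save-game Blueprint that holds the player's money and upgrade data for the pistol, assault rifle, shotgun and railgun.
; Each weapon has a stat map and a level map, and its update function adds to the named stat and increments that level, printing an error for unknown names.
; ResetUpgradeLevels returns levels to Level1 without touching stat values.
; BuyUpgrade deducts the truncated cost if affordable and reports success.
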(fn UpdatePistol
  (params (Name :type PistolUpgrades%20Enum :default "NewEnumerator0") (Value :type Float%20%28single-precision%29))
  (bind _pistol (Variables|Default|GetPistol))
  (bind _pistol_levels (Variables|Default|GetPistol_Levels))
  (bind (_value _returnvalue) (Utilities|Map|Find _pistol Name))
  (bind (_value_2 _returnvalue_2) (Utilities|Map|Find _pistol_levels Name))
  (if _returnvalue
    (Utilities|Map|Add _pistol Name (+ _value Value))
    (if _returnvalue_2
      (bind _result (Math|Float|IncrementFloat _value_2)
        (:%20%20
          (Utilities|Map|Add _pistol_levels Name _result)))
      (else
        (Development|PrintString 0 "Invalid Name!" :!label _label)))
    (else
      (goto _label))))

(fn UpdateRifle
  (params (Name :type RifleUpgrades%20Enum :default "NewEnumerator0") (Value :type Float%20%28single-precision%29))
  (bind _assault_rifle (Variables|Default|GetAssault%20Rifle))
  (bind _assault_rifle_levels (Variables|Default|GetAssault%20Rifle_Levels))
  (bind (_value _returnvalue) (Utilities|Map|Find _assault_rifle Name))
  (bind (_value_2 _returnvalue_2) (Utilities|Map|Find _assault_rifle_levels Name))
  (if _returnvalue
    (Utilities|Map|Add _assault_rifle Name (+ _value Value))
    (if _returnvalue_2
      (bind _result (Math|Float|IncrementFloat _value_2)
        (:%20%20
          (Utilities|Map|Add _assault_rifle_levels Name _result)))
      (else
        (Development|PrintString 0 "Invalid Name!" :!label _label)))
    (else
      (goto _label))))

(fn UpdateShotgun
  (params (Name :type ShotgunUpgrades%20Enum :default "NewEnumerator0") (Value :type Float%20%28single-precision%29))
  (bind _shotgun (Variables|Default|GetShotgun))
  (bind _shotgun_levels (Variables|Default|GetShotgun_Levels))
  (bind (_value _returnvalue) (Utilities|Map|Find _shotgun Name))
  (bind (_value_2 _returnvalue_2) (Utilities|Map|Find _shotgun_levels Name))
  (if _returnvalue
    (Utilities|Map|Add _shotgun Name (+ _value Value))
    (if _returnvalue_2
      (bind _result (Math|Float|IncrementFloat _value_2)
        (:%20%20
          (Utilities|Map|Add _shotgun_levels Name _result)))
      (else
        (Development|PrintString 0 "Invalid Name!" :!label _label)))
    (else
      (goto _label))))

(fn UpdateRailgun
  (params (Name :type RailgunUpgrades%20Enum :default "NewEnumerator0") (Value :type Float%20%28single-precision%29))
  (bind _railgun (Variables|Default|GetRailgun))
  (bind _railgun_levels (Variables|Default|GetRailgun_Levels))
  (bind (_value _returnvalue) (Utilities|Map|Find _railgun_levels Name))
  (bind (_value_2 _returnvalue_2) (Utilities|Map|Find _railgun Name))
  (if _returnvalue_2
    (Utilities|Map|Add _railgun Name (+ _value_2 Value))
    (if _returnvalue
      (bind _result (Math|Float|IncrementFloat _value)
        (:%20%20
          (Utilities|Map|Add _railgun_levels Name _result)))
      (else
        (Development|PrintString 0 "Invalid Name!" :!label _label)))
    (else
      (goto _label))))

(fn ResetUpgradeLevels
  (bind _pistol_levels (Variables|Default|GetPistol_Levels))
  (bind _assault_rifle_levels (Variables|Default|GetAssault%20Rifle_Levels))
  (bind _shotgun_levels (Variables|Default|GetShotgun_Levels))
  (bind _railgun_levels (Variables|Default|GetRailgun_Levels))
  (bind _level1 (LocalVariables|GetLevel1))
  (bind _values (Utilities|Map|Values _pistol_levels))
  (for (_ _array_index) _values
    (Utilities|Map|Add _pistol_levels (Utilities|Enum|ByteToEnumPistolUpgrades (Math|Conversions|ToByte(Integer) _array_index)) _level1))
  (bind _values_2 (Utilities|Map|Values _assault_rifle_levels))
  (for (_ _array_index_2) _values_2
    (Utilities|Map|Add _assault_rifle_levels (Utilities|Enum|ByteToEnumRifleUpgrades (Math|Conversions|ToByte(Integer) _array_index_2)) _level1))
  (bind _values_3 (Utilities|Map|Values _shotgun_levels))
  (for (_ _array_index_3) _values_3
    (Utilities|Map|Add _shotgun_levels (Utilities|Enum|ByteToEnumShotgunUpgrades (Math|Conversions|ToByte(Integer) _array_index_3)) _level1))
  (bind _values_4 (Utilities|Map|Values _railgun_levels))
  (for (_ _array_index_4) _values_4
    (Utilities|Map|Add _railgun_levels (Utilities|Enum|ByteToEnumRailgunUpgrades (Math|Conversions|ToByte(Integer) _array_index_4)) _level1)))

(fn BuyUpgrade
  (params (UpgradeCost :type Float%20%28single-precision%29))
  (bind _returnvalue (Math|Float|Truncate UpgradeCost))
  (if (>= (Variables|Default|GetMoney) _returnvalue)
    (LocalVariables|SetSuccess true)
    (Variables|Default|SetMoney (- (Variables|Default|GetMoney) _returnvalue))
    (else
      (LocalVariables|SetSuccess false)))
  (return (LocalVariables|GetSuccess)))