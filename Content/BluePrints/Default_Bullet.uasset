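; Default bullet projectile that damages insect and critter AI enemies on contact.
; Tick moves it along Direction at Speed using a swept location update, with no movement component.
; Box overlap runs a cast chain over spider, scorpion, centipede and snail, calling Death with Damage, except the snail, which receives zero.
; The bullet destroys itself after any overlap, printing a message for unidentified targets.
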(event OnComponentBeginOverlap(Box)
  (params (OverlappedComponent :type Primitive%20Component%20Object%20Reference) (OtherActor :type Actor%20Object%20Reference) (OtherComp :type Primitive%20Component%20Object%20Reference) (OtherBodyIndex :type Integer) (bFromSweep :type Boolean) (SweepResult :type Hit%20Result%20Structure%20%28by%20ref%29))
  (bind _damage (Variables|Default|GetDamage))
  (bind _asai_spider (Utilities|Casting|CastToAI_Spider OtherActor)
    (:then
      (Default|Death _asai_spider _damage))
    (:CastFailed
      (bind _asai_scorpion (Utilities|Casting|CastToAI_Scorpion OtherActor)
        (:then
          (Default|Death _asai_scorpion _damage))
        (:CastFailed
          (bind _asai_centipede (Utilities|Casting|CastToAI_Centipede OtherActor)
            (:then
              (Default|Death _asai_centipede _damage))
            (:CastFailed
              (bind _asai_snail (Utilities|Casting|CastToAI_Snail OtherActor)
                (:then
                  (Default|Death _asai_snail 0.0))
                (:CastFailed
                  (Development|PrintString "Unidentified target")))))))))
  (Actor|DestroyActor))

(event EventBeginPlay)

(event Collision|EventActorBeginOverlap
  (params (OtherActor :type Actor%20Object%20Reference)))

(event EventTick
  (params (DeltaSeconds :type Float%20%28single-precision%29))
  (Transformation|SetActorLocation (+ (Transformation|GetActorLocation self) (* (* (Variables|Default|GetDirection) (Variables|Default|GetSpeed)) DeltaSeconds)) true false))

(fn ConstructionScript)

(fn DestroySelf
  (CallFunction|DestroySelf))