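; Short-lived spawner actor that fires a shotgun spread of Shotgun_Bullet actors, then destroys itself.
; CalcSpawnValues scales the total angle by SpreadPower and adds a bullet for each full 0.2 of power above 1.
; ShootBullet offsets the aim by positive half that angle, then spawns bullets at further positive yaw steps, passing each its direction and damage.
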(event EventBeginPlay)

(event Collision|EventActorBeginOverlap
  (params (OtherActor :type Actor%20Object%20Reference)))

(event EventTick
  (params (DeltaSeconds :type Float%20%28single-precision%29)))

(event EventShootBullet
  (params (Direction :type Vector :default "0, 0, 0") (Bullet%20Speed :type Float%20%28single-precision%29) (Bulelt%20Size :type Float%20%28single-precision%29) (Bullet%20Damage :type Float%20%28single-precision%29) (SpreadPower :type Float%20%28single-precision%29))
  (CallFunction|CalcSpawnValues SpreadPower)
  (Variables|Default|SetStartDir (Math|Vector|RotateVector Direction (Math|Rotator|MakeRotator 0.0 0.0 (/ (Variables|Default|GetTotalAngle) 2.0))))
  (for _index (range 0 (Variables|Default|GetTotalBullets))
    (Game|SpawnActorfromClass "/Game/BluePrints/Shotgun_Bullet.Shotgun_Bullet_C" (Transformation|GetActorTransform self) "Undefined" 0 (Math|Vector|RotateVector (Variables|Default|GetStartDir) (Math|Rotator|MakeRotator 0.0 0.0 (* _index (Variables|Default|GetangleperBullet)))) 2e+01 Bullet%20Damage 7.0 0)
    (Development|PrintString "Shotgun Bullet spawned"))
  (Actor|DestroyActor))

(fn ConstructionScript)

(fn CalcSpawnValues
  (params (SpreadPower :type Float%20%28single-precision%29))
  (bind _returnvalue (- SpreadPower 1.0))
  (bind _output_get (Variables|Default|SetTotalAngle (* (Variables|Default|GetDefaultAngle) SpreadPower)))
  (bind _output_get_2 (Variables|Default|SetTotalBullets (+ (Variables|Default|GetDefaultBullets) (Math|Float|Truncate (/ (- _returnvalue (Math|Float|%(Float) _returnvalue 0.2)) 0.2)))))
  (Variables|Default|SetangleperBullet (/ _output_get (Math|Conversions|ToFloat(Integer) _output_get_2)))
  (return))