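; MenuSoundBoard is a Blueprint that plays menu button sounds through a single AudioComponent.
; Hover, Select and Back events each swap in their clip from the ButtonAudioClips array by index, play it and print a debug string.
; BeginPlay also starts the component playing, while UpdateAudioSettings is an empty stub.
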(event EventBeginPlay
  (Audio|Components|Audio|Play (Variables|Components|GetAudioComponent) 0.0))

(event EventTick
  (params (DeltaSeconds :type Float%20%28single-precision%29)))

(event EventHover
  (bind _audiocomponent (Variables|Components|GetAudioComponent))
  (Audio|Components|Audio|SetSound _audiocomponent (Utilities|Array|Get(acopy) (Variables|Default|GetButtonAudioClips)))
  (Audio|Components|Audio|Play _audiocomponent 0.0)
  (Development|PrintString "Hover noise"))

(event EventSelect
  (bind _audiocomponent (Variables|Components|GetAudioComponent))
  (Audio|Components|Audio|SetSound _audiocomponent (Utilities|Array|Get(acopy) (Variables|Default|GetButtonAudioClips) 1))
  (Audio|Components|Audio|Play _audiocomponent 0.0)
  (Development|PrintString "Select noise"))

(event EventBack
  (bind _audiocomponent (Variables|Components|GetAudioComponent))
  (Audio|Components|Audio|SetSound _audiocomponent (Utilities|Array|Get(acopy) (Variables|Default|GetButtonAudioClips) 2))
  (Audio|Components|Audio|Play _audiocomponent 0.0)
  (Development|PrintString "Back noise"))

(event EventUpdateAudioSettings)

(fn ConstructionScript)