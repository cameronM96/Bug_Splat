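; RailGun_Bullet is the railgun shot, an actor that damages enemy AI along a trace as soon as it spawns.
; On BeginPlay it runs a multi line trace on the Visibility channel, drawn for a debug duration, and loops over every hit.
; A chain of casts finds Spider, Scorpion, Centipede or Snail enemies and calls each one's Death with Damage; overlap and tick are unused.
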(event EventBeginPlay
  (bind _damage (Variables|Default|GetDamage))
  (bind (_outhits _returnvalue) (Collision|MultiLineTraceByChannel "0, 0, 0" "0, 0, 0" "TraceTypeQuery1" false 0 "ForDuration"))
  (if _returnvalue
    (for _array_element _outhits
      (bind _asai_spider (Utilities|Casting|CastToAI_Spider (.HitActor (Collision|BreakHitResult _array_element)))
        (:then
          (Default|Death _asai_spider _damage))
        (:CastFailed
          (bind _asai_scorpion (Utilities|Casting|CastToAI_Scorpion (.HitActor (Collision|BreakHitResult _array_element)))
            (:then
              (Default|Death _asai_scorpion _damage))
            (:CastFailed
              (bind _asai_centipede (Utilities|Casting|CastToAI_Centipede (.HitActor (Collision|BreakHitResult _array_element)))
                (:then
                  (Default|Death _asai_centipede _damage))
                (:CastFailed
                  (bind _asai_snail (Utilities|Casting|CastToAI_Snail (.HitActor (Collision|BreakHitResult _array_element))))
                  (Default|Death _asai_snail _damage))))))))))

(event Collision|EventActorBeginOverlap
  (params (OtherActor :type Actor%20Object%20Reference)))

(event EventTick
  (params (DeltaSeconds :type Float%20%28single-precision%29)))

(fn ConstructionScript)