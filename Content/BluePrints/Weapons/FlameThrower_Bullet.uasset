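; Flamethrower projectile that damages actors it overlaps and sets them on fire.
; ShootBullet sets direction, speed, damage and box scale, then Tick moves it with a swept location update and destroys it when its lifetime expires.
; Box overlap sends damage and timed fire messages, with fire damage scaled down from the hit damage, then destroys the bullet unless it touched a player character class.
; A Debugging flag self-fires it on BeginPlay.
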(event OnComponentBeginOverlap(Box)
  (params (OverlappedComponent :type Primitive%20Component%20Object%20Reference) (OtherActor :type Actor%20Object%20Reference) (OtherComp :type Primitive%20Component%20Object%20Reference) (OtherBodyIndex :type Integer) (bFromSweep :type Boolean) (SweepResult :type Hit%20Result%20Structure%20%28by%20ref%29))
  (bind _damage (Variables|Default|GetDamage))
  ;[1 1 1] Check Collision
  (Class|BPIAI|TakeDamage(Message) OtherActor _damage)
  (Class|BPIAI|SetFire(Message) OtherActor (/ _damage 4.0) 4.0)
  (Utilities|Casting|CastToThirdPersonCharacter OtherActor
    (:CastFailed
      (Utilities|Casting|CastToBP_Player1 OtherActor
        (:CastFailed
          (Actor|DestroyActor))))))

(event EventBeginPlay
  (bind _self self)
  (if (Variables|Default|GetDebugging)
    (Class|BPIShootBullet|ShootBullet(Message) _self (Transformation|GetActorForwardVector _self) 0.5 1.0 1.0 1.0)))

(event Collision|EventActorBeginOverlap
  (params (OtherActor :type Actor%20Object%20Reference)))

(event EventTick
  (params (DeltaSeconds :type Float%20%28single-precision%29))
  ;[1 1 1] Move Projectile
  (Transformation|SetActorLocation (+ (Transformation|GetActorLocation self) (* (* (Variables|Default|GetDirection) (Variables|Default|GetSpeed)) DeltaSeconds)) true false)
  ;[1 1 1] Check Life span
  (bind _output_get (Variables|Default|SetTimer (+ DeltaSeconds (Variables|Default|GetTimer))))
  (if (>= _output_get (Variables|Default|GetLifeTime))
    (Actor|DestroyActor)))

(event EventShootBullet
  (params (Direction :type Vector :default "0, 0, 0") (Bullet%20Speed :type Float%20%28single-precision%29) (Bulelt%20Size :type Float%20%28single-precision%29) (Bullet%20Damage :type Float%20%28single-precision%29) (SpreadPower :type Float%20%28single-precision%29))
  (bind _box (Variables|Default|GetBox))
  ;[1 1 1] Initialise
  (Variables|Default|SetDirection Direction)
  (Variables|Default|SetSpeed Bullet%20Speed)
  (Variables|Default|SetDamage Bullet%20Damage)
  (Transformation|SetWorldScale3D _box (* (Transformation|GetWorldScale _box) Bulelt%20Size))
  (Development|PrintString "FlameThrower Bullet Hello"))

(fn ConstructionScript)

(fn DestroySelf
  (CallFunction|DestroySelf))