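; Rail gun bullet actor that fires an instant piercing shot, damaging what it hits along a straight line.
; ShootBullet stores direction, damage and a size-scaled radius, then yaws the scene root, which carries the particle effect, toward the shot.
; A multi-sphere trace sends a TakeDamage message to each hit actor, and the actor destroys itself after a short delay.
; A Debugging flag self-fires on BeginPlay, and trace debug drawing stays persistent.
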(event Custom|Fire!
  (bind _direction (Variables|Default|GetDirection))
  (bind _scene (Variables|Default|GetScene))
  (bind _returnvalue (Transformation|GetWorldLocation _scene))
  ;[0.3419 0.4397 0.956] RotateParticle Effect in direction fired
  (Transformation|SetWorldRotation _scene (Math|Rotator|MakeRotator 0.0 0.0 (.Yaw (Math|Rotator|BreakRotator (Math|Rotator|FindLookatRotation _returnvalue (+ _direction _returnvalue))))) false false)
  ;[0 0.05951 0.3467] Find Hit Objects
  (bind _outhits (Collision|MultiSphereTraceByChannel _returnvalue (+ _returnvalue (* _direction 1e+03)) (Variables|Default|GetRadius) "TraceTypeQuery3" false 0 "Persistent"))
  (Development|PrintString (Utilities|String|ToString(Integer) (Utilities|Array|Length _outhits)))
  (if (> (Utilities|Array|Length _outhits) 0)
    ;[1 0.003851 0] Damage enemy
    (for _array_element _outhits
      (Class|BPIAI|TakeDamage(Message) (.HitActor (Collision|BreakHitResult _array_element)) (Variables|Default|GetDamage))))
  (Utilities|FlowControl|Delay 2.0)
  (Actor|DestroyActor))

(event EventShootBullet
  (params (Direction :type Vector :default "0, 0, 0") (Bullet%20Speed :type Float%20%28single-precision%29) (Bulelt%20Size :type Float%20%28single-precision%29) (Bullet%20Damage :type Float%20%28single-precision%29) (SpreadPower :type Float%20%28single-precision%29))
  ;[0.05781 0.227 0.3419] Initialise
  (Variables|Default|SetDirection Direction)
  (Variables|Default|SetDamage Bullet%20Damage)
  (Variables|Default|SetRadius (* Bulelt%20Size 25.0))
  (CallFunction|Fire!)
  (Development|PrintString "Hello"))

(event EventBeginPlay
  (bind _self self)
  (if (Variables|Default|GetDebugging)
    (Class|BPIShootBullet|ShootBullet(Message) _self (Transformation|GetActorForwardVector _self) 1.0 1.0 1e+01 1.0)))

(fn ConstructionScript)