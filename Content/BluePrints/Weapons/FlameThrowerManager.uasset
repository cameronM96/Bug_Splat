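; Flamethrower weapon actor that plays a flame effect and fires a damaging FlameThrower_Bullet on each shot.
; ShootBullet stores speed and damage, scales the scene, activates the effect and spawns the projectile along the actor's forward vector.
; Tick counts down the lifetime to switch the effect off; in Debugging mode it then rotates and refires, starting from BeginPlay.
; Destroy clears the owner and removes the actor after a short delay.
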(event Custom|Destroy
  (Actor|SetOwner self 0)
  (Utilities|FlowControl|Delay 3.0)
  (Actor|DestroyActor))

(event EventBeginPlay
  (bind _self self)
  (Components|Activation|Deactivate (Variables|Default|GetFlamethrower))
  (if (Variables|Default|GetDebugging)
    (Class|BPIShootBullet|ShootBullet(Message) _self (Transformation|GetActorForwardVector _self) 0.95 1.0 2.0 1.0)))

(event Collision|EventActorBeginOverlap
  (params (OtherActor :type Actor%20Object%20Reference)))

(event EventTick
  (params (DeltaSeconds :type Float%20%28single-precision%29))
  (bind _self self)
  (bind _returnvalue (Transformation|GetActorRotation _self))
  (bind (_roll _pitch _yaw) (Math|Rotator|BreakRotator _returnvalue))
  (if (Components|Activation|IsActive (Variables|Default|GetFlamethrower))
    (bind _output_get (Variables|Default|SetTimer (- (Variables|Default|GetTimer) DeltaSeconds)))
    (if (<= _output_get 0.0)
      (Components|Activation|Deactivate (Variables|Default|GetFlamethrower))
      (if (Variables|Default|GetDebugging)
        (Utilities|FlowControl|Delay 0.0)
        (Transformation|SetActorRotation _self (Math|Rotator|MakeRotator _roll _pitch (+ _yaw 15.0)))
        (Class|BPIShootBullet|ShootBullet(Message) self (Variables|Default|GetDirection) 0.95 1.0 (Variables|Default|GetDamage) 0.0)))))

(event EventShootBullet
  (params (Direction :type Vector :default "0, 0, 0") (Bullet%20Speed :type Float%20%28single-precision%29) (Bulelt%20Size :type Float%20%28single-precision%29) (Bullet%20Damage :type Float%20%28single-precision%29) (SpreadPower :type Float%20%28single-precision%29))
  ;[1 1 1] Initialise
  (Variables|Default|SetDirection Direction)
  (Variables|Default|SetSpeed (* Bullet%20Speed 5e+02))
  (Variables|Default|SetDamage Bullet%20Damage)
  (Transformation|SetWorldScale3D (Variables|Default|GetScene) (* "1.000000,1.000000,1.000000" Bulelt%20Size))
  (Components|Activation|Activate (Variables|Default|GetFlamethrower) false)
  (Variables|Default|SetTimer (Variables|Default|GetLifeTime))
  (Game|SpawnActorfromClass "/Game/BluePrints/Weapons/FlameThrower_Bullet.FlameThrower_Bullet_C" (Transformation|GetWorldTransform (Variables|Default|GetScene1)) "Undefined" 0 (Transformation|GetActorForwardVector self) (Variables|Default|GetSpeed) (Variables|Default|GetDamage) 2.0 0))

(fn ConstructionScript)

(fn DestroySelf
  (CallFunction|DestroySelf))