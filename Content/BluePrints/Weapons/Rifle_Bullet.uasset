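; Rifle projectile Blueprint that flies along a given direction and damages actors it overlaps.
; ShootBullet sets direction, damage and scaled speed, then Tick moves it with a swept location update until its lifetime expires.
; The intended inaccuracy adds Perlin noise to Z, but samples a constant input, so the offset never varies.
; Box overlap sends damage to any actor, then destroys the bullet unless that actor is a ThirdPersonCharacter or BP_Player1.
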(event OnComponentBeginOverlap(Box)
  (params (OverlappedComponent :type Primitive%20Component%20Object%20Reference) (OtherActor :type Actor%20Object%20Reference) (OtherComp :type Primitive%20Component%20Object%20Reference) (OtherBodyIndex :type Integer) (bFromSweep :type Boolean) (SweepResult :type Hit%20Result%20Structure%20%28by%20ref%29))
  ;[1 1 1] Check Collision
  (Class|BPIAI|TakeDamage(Message) OtherActor (Variables|Default|GetDamage))
  (Utilities|Casting|CastToThirdPersonCharacter OtherActor
    (:CastFailed
      (Utilities|Casting|CastToBP_Player1 OtherActor
        (:CastFailed
          (Actor|DestroyActor))))))

(event EventBeginPlay
  (bind _self self)
  (if (Variables|Default|GetDebugging)
    (Class|BPIShootBullet|ShootBullet(Message) _self (Transformation|GetActorForwardVector _self) 1.0 1.0 1.0 1.0)))

(event Collision|EventActorBeginOverlap
  (params (OtherActor :type Actor%20Object%20Reference)))

(event EventTick
  (params (DeltaSeconds :type Float%20%28single-precision%29))
  (bind _direction (Variables|Default|GetDirection))
  (bind (_x _y _z) (Math|Vector|BreakVector _direction))
  ;[1 1 1] Move Projectile
  (Transformation|SetActorLocation (+ (Transformation|GetActorLocation self) (* (* (Math|Vector|MakeVector _x _y (+ _z (Class|KismetMathLibrary|PerlinNoise1D 1e+01))) (Variables|Default|GetSpeed)) DeltaSeconds)) true false)
  ;[1 1 1] Check Life span
  (bind _output_get (Variables|Default|SetTimer (+ DeltaSeconds (Variables|Default|GetTimer))))
  (if (>= _output_get (Variables|Default|GetLifeTime))
    (Actor|DestroyActor)))

(event EventShootBullet
  (params (Direction :type Vector :default "0, 0, 0") (Bullet%20Speed :type Float%20%28single-precision%29) (Bulelt%20Size :type Float%20%28single-precision%29) (Bullet%20Damage :type Float%20%28single-precision%29) (SpreadPower :type Float%20%28single-precision%29))
  (Variables|Default|SetDirection Direction)
  (Variables|Default|SetSpeed (* Bullet%20Speed 5e+02))
  (Variables|Default|SetDamage Bullet%20Damage)
  (Development|PrintString "Rifle Hello"))

(fn ConstructionScript)

(fn DestroySelf
  (CallFunction|DestroySelf))