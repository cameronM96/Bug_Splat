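; Short-lived shotgun spawner actor that fires a horizontal fan of Shotgun_Bullet actors around a given direction, then destroys itself.
; CalcSpawnValues scales the fan angle with SpreadPower and adds pellets in stepped increments as spread grows.
; ShootBullet rotates the direction back half the fan in 2D, then spawns bullets at evenly stepped yaw offsets, passing each the damage and a fixed speed.
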(event EventBeginPlay)

(event EventShootBullet
  (params (Direction :type Vector :default "0, 0, 0") (Bullet%20Speed :type Float%20%28single-precision%29) (Bulelt%20Size :type Float%20%28single-precision%29) (Bullet%20Damage :type Float%20%28single-precision%29) (SpreadPower :type Float%20%28single-precision%29))
  ;[1 1 1] Find Start direction
  (CallFunction|CalcSpawnValues SpreadPower)
  (bind _newdir (CallFunction|RotateAboutPoint Direction (* (/ (Variables|Default|GetTotalAngle) 2.0) -1.0)))
  (Variables|Default|SetStartDir _newdir)
  (for _index (range 0 (Variables|Default|GetTotalBullets))
    (Game|SpawnActorfromClass "/Game/BluePrints/Weapons/Shotgun_Bullet.Shotgun_Bullet_C" (Transformation|GetActorTransform self) "Undefined" 0 (Math|Vector|RotateVector (Variables|Default|GetStartDir) (Math|Rotator|MakeRotator 0.0 0.0 (* _index (Variables|Default|GetangleperBullet)))) 2e+02 Bullet%20Damage 7.0 0)
    (Development|PrintString "Shotgun Bullet spawned"))
  (Actor|DestroyActor))

(fn ConstructionScript)

(fn CalcSpawnValues
  (params (SpreadPower :type Float%20%28single-precision%29))
  (bind _returnvalue (- SpreadPower 1.0))
  (bind _output_get (Variables|Default|SetTotalAngle (* (Variables|Default|GetDefaultAngle) SpreadPower)))
  (bind _output_get_2 (Variables|Default|SetTotalBullets (+ (Variables|Default|GetDefaultBullets) (Math|Float|Truncate (/ (- _returnvalue (Math|Float|%(Float) _returnvalue 0.2)) 0.2)))))
  (Variables|Default|SetangleperBullet (/ _output_get (Math|Conversions|ToFloat(Integer) _output_get_2)))
  (return))

(fn RotateAboutPoint
  (params (Point :type Vector) (Angle :type Float%20%28single-precision%29))
  (bind (_x _y) (Math|Vector|BreakVector Point))
  (bind _returnvalue (Math|Trig|Cos(Degrees) Angle))
  (bind _returnvalue_2 (Math|Trig|Sin(Degrees) Angle))
  (return (Math|Vector|MakeVector (- (* _x _returnvalue) (* _y _returnvalue_2)) (+ (* _y _returnvalue) (* _x _returnvalue_2)) 0.0)))