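; GameSoundBoard is a Blueprint that serves as a central player for game sounds.
; AudioComponent starts playing on BeginPlay, while a separate ButtonAudio component handles event-driven sounds.
; SetWeapon loads a clip from WeaponAudioClips into ButtonAudio for PlayWeapon to play; PlayerDeath swaps in the death sound and plays it immediately.
; The UpdateAudioSettings event is an empty stub.
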(event EventBeginPlay
  (Audio|Components|Audio|Play (Variables|Components|GetAudioComponent) 0.0))

(event EventTick
  (params (DeltaSeconds :type Float%20%28single-precision%29)))

(event EventSetWeapon
  (params (Weapon# :type Integer))
  (Audio|Components|Audio|SetSound (Variables|Default|GetButtonAudio) (Utilities|Array|Get(acopy) (Variables|Default|GetWeaponAudioClips) Weapon#)))

(event EventPlayWeapon
  (Audio|Components|Audio|Play (Variables|Default|GetButtonAudio) 0.0))

(event EventPlayerDeath
  (bind _buttonaudio (Variables|Default|GetButtonAudio))
  (Audio|Components|Audio|SetSound _buttonaudio "/Game/Audio/EffectSounds/PlayerDeath.PlayerDeath")
  (Audio|Components|Audio|Play _buttonaudio 0.0))

(event EventUpdateAudioSettings)

(fn ConstructionScript)