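; Shotgun bullet projectile that flies in a straight line and deals damage to what it overlaps.
; Tick moves it with a swept SetActorLocation along Direction at Speed and destroys it once its timer reaches LifeTime.
; Box overlap sends TakeDamageMessage to any actor, but destroys the bullet only when that actor is a ThirdPersonCharacter.
; A separate DestroySelf function only calls DestroySelf and is unused by the event graph.
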(event OnComponentBeginOverlap(Box)
  (params (OverlappedComponent :type Primitive%20Component%20Object%20Reference) (OtherActor :type Actor%20Object%20Reference) (OtherComp :type Primitive%20Component%20Object%20Reference) (OtherBodyIndex :type Integer) (bFromSweep :type Boolean) (SweepResult :type Hit%20Result%20Structure%20%28by%20ref%29))
  ;[1 1 1] Check Collision
  (Class|BPIAI|TakeDamage(Message) OtherActor (Variables|Default|GetDamage))
  (Utilities|Casting|CastToThirdPersonCharacter OtherActor)
  (Actor|DestroyActor))

(event EventBeginPlay)

(event Collision|EventActorBeginOverlap
  (params (OtherActor :type Actor%20Object%20Reference)))

(event EventTick
  (params (DeltaSeconds :type Float%20%28single-precision%29))
  ;[1 1 1] Move Projectile
  (Transformation|SetActorLocation (+ (Transformation|GetActorLocation self) (* (* (Variables|Default|GetDirection) (Variables|Default|GetSpeed)) DeltaSeconds)) true false)
  ;[1 1 1] Check Life span
  (bind _output_get (Variables|Default|SetTimer (+ DeltaSeconds (Variables|Default|GetTimer))))
  (if (>= _output_get (Variables|Default|GetLifeTime))
    (Actor|DestroyActor)))

(fn ConstructionScript)

(fn DestroySelf
  (CallFunction|DestroySelf))