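; BP_Cyborg is a player cyborg Blueprint, kept in a FailedTest folder, that drives a walk animation from keyboard input.
; BeginPlay caches the skeletal mesh's Cyborg_Animation_State anim instance.
; W (bound twice), A and S presses set walk flags through a Cyborg reference, with no release handling or movement logic.
; Tick copies WalkAnimation and StopWalk into the anim instance's Go and NotWalk booleans.
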(event EventBeginPlay
  (bind _ascyborg_animation_state (Utilities|Casting|CastToCyborg_Animation_State (Components|SkeletalMesh|GetAnimInstance (Variables|Default|GetSkeletalMesh))))
  (Variables|Default|SetCyborgAnimationState _ascyborg_animation_state)
  (Variables|Default|SetActive true))

(event Collision|EventActorBeginOverlap
  (params (OtherActor :type Actor%20Object%20Reference)))

(event EventTick
  (params (DeltaSeconds :type Float%20%28single-precision%29))
  (bind _cyborganimationstate (Variables|Default|GetCyborgAnimationState))
  (Utilities|FlowControl|Sequence
    (:then_0
      (if (Variables|Default|GetWalkAnimation)
        (Variables|/Game/Assests/Player/Player1/FailedTest/Cyborg_Animation_State.Cyborg_Animation_State_C|SetGo _cyborganimationstate true)
        (else
          (Variables|/Game/Assests/Player/Player1/FailedTest/Cyborg_Animation_State.Cyborg_Animation_State_C|SetGo _cyborganimationstate false))))
    (:then_1
      (if (Variables|Default|GetStopWalk)
        (Variables|/Game/Assests/Player/Player1/FailedTest/Cyborg_Animation_State.Cyborg_Animation_State_C|SetNotWalk _cyborganimationstate true)
        (else
          (Variables|/Game/Assests/Player/Player1/FailedTest/Cyborg_Animation_State.Cyborg_Animation_State_C|SetNotWalk _cyborganimationstate false))))))

(event Input|KeyboardEvents|W
  (params (Key :type Key%20Structure))
  (bind _cyborg (Variables|Default|GetCyborg))
  (:Pressed
    (Variables|BP_Cyborg_C|SetWalkAnimation _cyborg true)
    (Variables|BP_Cyborg_C|SetStopWalk _cyborg false)))

(event Input|KeyboardEvents|W
  (params (Key :type Key%20Structure))
  (bind _cyborg (Variables|Default|GetCyborg))
  (:Pressed
    (Variables|BP_Cyborg_C|SetWalkAnimation _cyborg true)
    (Variables|BP_Cyborg_C|SetStopWalk _cyborg false)))

(event Input|KeyboardEvents|A
  (params (Key :type Key%20Structure))
  (bind _cyborg (Variables|Default|GetCyborg))
  (:Pressed
    (Variables|BP_Cyborg_C|SetWalkAnimation _cyborg true)
    (Variables|BP_Cyborg_C|SetStopWalk _cyborg false)))

(event Input|KeyboardEvents|S
  (params (Key :type Key%20Structure))
  (bind _cyborg (Variables|Default|GetCyborg))
  (:Pressed
    (Variables|BP_Cyborg_C|SetWalkAnimation _cyborg true)
    (Variables|BP_Cyborg_C|SetStopWalk _cyborg false)))

(fn ConstructionScript)