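; BP_Cyborg is a Player 1 cyborg Blueprint that drives the walk animation of its skeletal mesh.
; Shortly after BeginPlay it caches the mesh's ANIM_BP_Cyborg_Walk instance and sets an Active flag.
; While active, Tick switches the anim instance's AnimBlendTarget between walking and zero based on the WalkAnimation flag, which this Blueprint only reads.
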(event EventBeginPlay
  (Utilities|FlowControl|Delay 0.2)
  (bind _asanim_bp_cyborg_walk (Utilities|Casting|CastToANIM_BP_Cyborg_Walk (Components|SkeletalMesh|GetAnimInstance (Variables|Default|GetSkeletalMesh))))
  (Variables|Default|SetAnimation _asanim_bp_cyborg_walk)
  (Variables|Default|SetActive true))

(event Collision|EventActorBeginOverlap
  (params (OtherActor :type Actor%20Object%20Reference)))

(event EventTick
  (params (DeltaSeconds :type Float%20%28single-precision%29))
  (bind _animation (Variables|Default|GetAnimation))
  (if (Variables|Default|GetActive)
    (if (Variables|Default|GetWalkAnimation)
      (Variables|/Game/Assests/Player/Player1/ANIM_BP_Cyborg_Walk.ANIM_BP_Cyborg_Walk_C|SetAnimBlendTarget _animation 25.0)
      (else
        (Variables|/Game/Assests/Player/Player1/ANIM_BP_Cyborg_Walk.ANIM_BP_Cyborg_Walk_C|SetAnimBlendTarget _animation 0.0)))))

(fn ConstructionScript)