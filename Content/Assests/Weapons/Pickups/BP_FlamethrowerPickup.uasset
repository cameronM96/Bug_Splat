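; Flamethrower weapon pickup that spins its sphere and reacts when BP_Player1 overlaps it.
; On overlap it loads the "Default" save slot and relays the save and a cast-failed flag through PickupTriggerServer to PickupTriggerMulti.
; That event sends EquipNewGunMessage with saved FlameThrower stats only when CastFailed is true, the path given no save object, then destroys the pickup either way.
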(event OnComponentBeginOverlap(Sphere)
  (params (OverlappedComponent :type Primitive%20Component%20Object%20Reference) (OtherActor :type Actor%20Object%20Reference) (OtherComp :type Primitive%20Component%20Object%20Reference) (OtherBodyIndex :type Integer) (bFromSweep :type Boolean) (SweepResult :type Hit%20Result%20Structure%20%28by%20ref%29))
  (bind _asbp_player_1 (Utilities|Casting|CastToBP_Player1 OtherActor))
  (if (== _asbp_player_1 OtherActor)
    (bind _returnvalue (SaveGame|LoadGamefromSlot "Default"))
    (bind _assave_game_bp (Utilities|Casting|CastToSave_Game_BP _returnvalue)
      (:then
        (CallFunction|PickupTriggerServer _assave_game_bp false))
      (:CastFailed
        (CallFunction|PickupTriggerServer 0 true)))))

(event Custom|PickupTriggerMulti
  (params (SaveGameFile :type Save%20Game%20BP%20Object%20Reference) (CastFailed :type Boolean))
  (bind _flamethrower (Variables|/Game/BluePrints/Save_Game_BP.Save_Game_BP_C|GetFlameThrower SaveGameFile))
  (if CastFailed
    (Class|BPIPickupSystem|EquipNewGun(Message) (stale OnComponentBeginOverlap(Sphere) OtherActor) (.Value (Utilities|Map|Find _flamethrower "NewEnumerator1")) (.Value (Utilities|Map|Find _flamethrower "")) 0.0 (.Value (Utilities|Map|Find _flamethrower "NewEnumerator2")) (Math|Float|Truncate (.Value (Utilities|Map|Find _flamethrower "NewEnumerator3"))) false "/Game/BluePrints/Weapons/FlameThrowerManager.FlameThrowerManager_C" 4))
  (Actor|DestroyActor))

(event Custom|PickupTriggerServer
  (params (SaveGame :type Save%20Game%20BP%20Object%20Reference) (CastFailed :type Boolean))
  (CallFunction|PickupTriggerMulti SaveGame CastFailed))

(event EventTick
  (params (DeltaSeconds :type Float%20%28single-precision%29))
  (Transformation|AddLocalRotation (Variables|Default|GetSphere) (Math|Rotator|MakeRotator 0.0 0.0 (Variables|Default|GetRotation%20Speed)) false false))

(fn ConstructionScript)