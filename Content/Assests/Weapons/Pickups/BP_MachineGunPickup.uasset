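; Machine gun pickup that spins its sphere every tick and equips the player with a rifle when overlapped.
; On overlap by BP_Player1, it reads fire rate, damage, bullet speed and ammo from the AssaultRifle map in the GameModeController's save game.
; It passes these with the rifle bullet type through EquipNewGunMessage to the player, then destroys itself.
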(event OnComponentBeginOverlap(Sphere)
  (params (OverlappedComponent :type Primitive%20Component%20Object%20Reference) (OtherActor :type Actor%20Object%20Reference) (OtherComp :type Primitive%20Component%20Object%20Reference) (OtherBodyIndex :type Integer) (bFromSweep :type Boolean) (SweepResult :type Hit%20Result%20Structure%20%28by%20ref%29))
  (bind _asbp_player_1 (Utilities|Casting|CastToBP_Player1 OtherActor))
  (if (== _asbp_player_1 OtherActor)
    (bind _asgame_mode_controller (Utilities|Casting|CastToGameModeController (Game|GetGameMode)))
    (Class|BPIPickupSystem|EquipNewGun(Message) OtherActor (.Value (Utilities|Map|Find (Variables|/Game/BluePrints/Save_Game_BP.Save_Game_BP_C|GetAssault%20Rifle (Variables|/Game/BluePrints/GameModeController.GameModeController_C|GetSaveGameFile _asgame_mode_controller)) "NewEnumerator1")) (.Value (Utilities|Map|Find (Variables|/Game/BluePrints/Save_Game_BP.Save_Game_BP_C|GetAssault%20Rifle (Variables|/Game/BluePrints/GameModeController.GameModeController_C|GetSaveGameFile _asgame_mode_controller)) "")) 1.0 (.Value (Utilities|Map|Find (Variables|/Game/BluePrints/Save_Game_BP.Save_Game_BP_C|GetAssault%20Rifle (Variables|/Game/BluePrints/GameModeController.GameModeController_C|GetSaveGameFile _asgame_mode_controller)) "NewEnumerator2")) (Math|Float|Truncate (.Value (Utilities|Map|Find (Variables|/Game/BluePrints/Save_Game_BP.Save_Game_BP_C|GetAssault%20Rifle (Variables|/Game/BluePrints/GameModeController.GameModeController_C|GetSaveGameFile _asgame_mode_controller)) "NewEnumerator3"))) false "/Game/BluePrints/Rifle_Bullet.Rifle_Bullet_C" 1)
    (Actor|DestroyActor)))

(event EventTick
  (params (DeltaSeconds :type Float%20%28single-precision%29))
  (Transformation|AddLocalRotation (Variables|Default|GetSphere) (Math|Rotator|MakeRotator 0.0 0.0 (Variables|Default|GetRotation%20Speed)) false false))

(fn ConstructionScript)